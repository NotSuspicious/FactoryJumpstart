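; Player character for a factory game that fires retractable left and right clamps and interacts with tutorial cartridges, levers and level exits.
; Each shoot event spawns a clamp with its cable attached to the wrist, or releases the existing one.
; Interacting with a cartridge shows dialogue, disables movement and blocks shooting.
; Tick traces down from each foot socket and interpolates scale-adjusted IK offsets for foot placement.
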(event `self.ReceiveBeginPlay`
  (bind _returnvalue (`|CreateWidget` "/Game/Blueprints/UI/UW_DialogueUI.UW_DialogueUI_C"))
  (bind _output_get (set `self.dialogueWidget` _returnvalue))
  (`UserWidget.AddToViewport` _output_get 0)
  (`Widget.SetVisibility` _output_get "Hidden"))

(event `self.ReceiveTick`
  (params (DeltaSeconds :type "Float (single-precision)"))
  ; Update IK OFfset
  (bind _ikoffset (`self.IKFootTrace` "RightFootSocket" (`self.IKTraceDistance`)))
  (set `self.IKOffsetRightFoot` (`KismetMathLibrary.FInterpTo` (`self.IKOffsetRightFoot`) _ikoffset DeltaSeconds (`self.IKInterpSpeed`)))
  (bind _ikoffset_2 (`self.IKFootTrace` "LeftFootSocket" (`self.IKTraceDistance`)))
  (set `self.IKOffsetLeftFoot` (`KismetMathLibrary.FInterpTo` (`self.IKOffsetLeftFoot`) _ikoffset_2 DeltaSeconds (`self.IKInterpSpeed`))))

(event `/Game/Blueprints/BPI_FactoryPlayerActions.OnLeftShoot`
  (if (`self.dialogueMode?`)
    _
    (elif (`KismetSystemLibrary.IsValid` (`self.LeftClampInstance`))
      (`GameplayStatics.PlaySound2D` "/Game/Audio/SFX/Clamp_Retracting_v2.Clamp_Retracting_v2" 1.0 1.0 0.0 null null)
      (`ClampProjectile.Release` (`self.LeftClampInstance`))
      (else
        (`GameplayStatics.PlaySound2D` "/Game/Audio/SFX/Clamp_Shooting_Out_v2.Clamp_Shooting_Out_v2" 1.0 1.0 0.0 null null)
        (bind _returnvalue (`|SpawnActorFromClass` "/Game/Blueprints/BP_LeftClamp.BP_LeftClamp_C" (`KismetMathLibrary.MakeTransform` (`SceneComponent.GetSocketLocation` (`self.Mesh`) "Wrist_L") (`SceneComponent.K2_GetComponentRotation` (`self.CapsuleComponent`))) "Undefined" "MultiplyWithRoot" null null))
        (bind _output_get (set `self.LeftClampInstance` _returnvalue))
        (`SceneComponent.K2_AttachToComponent` (`ClampProjectile.Cable` _output_get) (`self.Mesh`) "Wrist_L" "KeepRelative" "KeepRelative" "KeepRelative" true)))))

(event `/Game/Blueprints/BPI_FactoryPlayerActions.OnRightShoot`
  (if (`self.dialogueMode?`)
    _
    (elif (`KismetSystemLibrary.IsValid` (`self.RightClampInstance`))
      (`GameplayStatics.PlaySound2D` "/Game/Audio/SFX/Clamp_Retracting_v2.Clamp_Retracting_v2" 1.0 1.0 0.0 null null)
      (`ClampProjectile.Release` (`self.RightClampInstance`))
      (else
        (`GameplayStatics.PlaySound2D` "/Game/Audio/SFX/Clamp_Shooting_Out_v2.Clamp_Shooting_Out_v2" 1.0 1.0 0.0 null null)
        (bind _returnvalue (`|SpawnActorFromClass` "/Game/Blueprints/BP_RightClamp.BP_RightClamp_C" (`KismetMathLibrary.MakeTransform` (`SceneComponent.GetSocketLocation` (`self.Mesh`) "Wrist_R") (`SceneComponent.K2_GetComponentRotation` (`self.CapsuleComponent`))) "Undefined" "MultiplyWithRoot" null null))
        (bind _output_get (set `self.RightClampInstance` _returnvalue))
        (`SceneComponent.K2_AttachToComponent` (`ClampProjectile.Cable` _output_get) (`self.Mesh`) "Wrist_R" "KeepRelative" "KeepRelative" "KeepRelative" true)))))

(event `/Game/Blueprints/BPI_FactoryPlayerActions.OnInteract`
  (bind _tutorialcartridge (`self.tutorialCartridge`))
  (bind _levelexit (`self.levelExit`))
  (`/Engine/EditorBlueprintResources/StandardMacros.IsValid` _tutorialcartridge
    (:`Is Valid`
      (`/Game/Blueprints/MechanicalObjects/BP_TutorialCartridge.PrintDialogue` _tutorialcartridge (`self.dialogueWidget`))
      (`ActorComponent.Deactivate` (`self.CharacterMovement`))
      (set `self.dialogueMode?` true))
    (:`Is Not Valid`
      (`/Engine/EditorBlueprintResources/StandardMacros.IsValid` (`self.currentLever`)
        (:`Is Valid`
          (if (`self.canUseLever?`)
            (`/Game/Blueprints/MechanicalObjects/BP_Lever.ActivateEject` (`self.currentLever`))))
        (:`Is Not Valid`
          (`/Engine/EditorBlueprintResources/StandardMacros.IsValid` _levelexit
            (:`Is Valid`
              (`/Game/Blueprints/WinCondition/BP_LevelExitDoor.NextLevel` _levelexit))))))))

(fn `IKFootTrace`
  (params (Socket :type Name) (TraceDistance :type "Float (double-precision)"))
  (returns (IKOffset :type "Float (double-precision)"))
  (bind (_returnvalue_x _returnvalue_y _returnvalue_z) (`KismetMathLibrary.BreakVector` (`self.K2_GetActorLocation`)))
  (bind (_returnvalue_x_2 _returnvalue_y_2) (`KismetMathLibrary.BreakVector` (`SceneComponent.GetSocketLocation` (`self.Mesh`) Socket)))
  (bind _returnvalue (`KismetMathLibrary.MakeVector` _returnvalue_x_2 _returnvalue_y_2 (- _returnvalue_z TraceDistance)))
  (bind (_outhit _returnvalue_2) (`KismetSystemLibrary.LineTraceSingle` :`Start` (`KismetMathLibrary.MakeVector` _returnvalue_x_2 _returnvalue_y_2 _returnvalue_z) :`End` _returnvalue :`TraceChannel` "TraceTypeQuery1" :`bTraceComplex` true :`DrawDebugType` "ForOneFrame"))
  (return (`KismetMathLibrary.SelectFloat` (/ (`KismetMathLibrary.VSize` (- _returnvalue (`.Location` (`GameplayStatics.BreakHitResult` _outhit)))) (`self.Height`)) 0.0 _returnvalue_2)))

(fn `UserConstructionScript`
  (set `self.Height` (.z (.scale (`self.GetTransform`)))))