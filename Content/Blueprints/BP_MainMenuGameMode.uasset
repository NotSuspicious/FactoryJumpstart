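; Main menu game mode that sets up the start screen when the level begins.
; On BeginPlay it plays a slide open transition through the level transition subsystem and starts the Intro level sequence, whose finish event starts an endlessly looping Loop sequence.
; It also creates the StartMenu widget, shows the mouse cursor and switches the player to UI-only input.
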(event `PlayLoop`
  ; Sequence
  (`LevelSequencePlayer.CreateLevelSequencePlayer` (`self.Loop`) (make `MovieSceneSequencePlaybackSettings` true (make `MovieSceneSequenceLoopCount` -1))))

(event `self.ReceiveBeginPlay`
  (bind _returnvalue (`GameplayStatics.GetPlayerController` 0))
  (`LevelTransitionSubsystem.PlayOpenTransition` (subsystem `LevelTransitionSubsystem`) (make `SlideTransitionSettings` (struct :`A` 1.0) "LeftToRight" "EaseInOut" 2.0 null 1.0 1.0) null)
  ; Sequence
  (bind (_outactor _returnvalue_2) (`LevelSequencePlayer.CreateLevelSequencePlayer` (`self.Intro`) (make `MovieSceneSequencePlaybackSettings` true)))
  (add `MovieSceneSequencePlayer.OnFinished` _returnvalue_2 (delegate `PlayLoop`))
  (bind _returnvalue_3 (`|CreateWidget` "/Game/UI/StartMenu.StartMenu_C"))
  (`UserWidget.AddToViewport` _returnvalue_3 0)
  (set `PlayerController.bShowMouseCursor` true _returnvalue)
  (`WidgetBlueprintLibrary.SetInputMode_UIOnlyEx` _returnvalue null))

(fn `UserConstructionScript`)