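; Battery compartment that takes a battery from the player and powers a linked treadmill or HandyBot.
; Overlapping the box in the matching carry state fills the empty slot, showing the battery mesh and resetting that state.
; With red and black clamps connected, a filled compartment charges once, starting the treadmill's charge cycle and sounds or activating the robot.
; Unloading empties the slot and launches a new BP_Battery along the arrow.
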(event `self.ReceiveBeginPlay`
  (`|ExecutionSequence`
    (:`then_0`
      (`/Engine/EditorBlueprintResources/StandardMacros.IsValid` (`self.treadmillObj`)
        (:`Is Valid`
          (set `self.objectAttachment` "NewEnumerator0"))
        (:`Is Not Valid`
          (`/Engine/EditorBlueprintResources/StandardMacros.IsValid` (`self.handyBotObj`)
            (:`Is Valid`
              (set `self.objectAttachment` "NewEnumerator1"))))))
    (:`then_1`
      (set `self.compartmentState` "NewEnumerator0")
      (`SceneComponent.SetVisibility` (`self.PSCP_Game_Jam_battery`) false false))))

(event `self.Box.OnComponentBeginOverlap`
  (params (OverlappedComponent :type "PrimitiveComponent Object Reference") (OtherActor :type "Actor Object Reference") (OtherComp :type "PrimitiveComponent Object Reference") (OtherBodyIndex :type Integer) (bFromSweep :type Boolean) (SweepResult :type "HitResult Structure (by ref)"))
  (bind _asbp_factory_character (cast `/Game/Blueprints/BP_FactoryCharacter` OtherActor))
  (if (`|EnumEquality` (`/Game/Blueprints/BP_FactoryCharacter.playerCarryState` _asbp_factory_character) "NewEnumerator1")
    (if (`|EnumEquality` (`self.compartmentState`) "NewEnumerator0")
      (`GameplayStatics.PlaySound2D` "/Game/Audio/SFX/Putting_Item_in_Slot___Discard.Putting_Item_in_Slot___Discard" 1.0 1.0 0.0 null null)
      (set `self.compartmentState` "NewEnumerator1")
      (`SceneComponent.SetVisibility` (`self.PSCP_Game_Jam_battery`) true false)
      (bind _asbp_factory_character_2 (cast `/Game/Blueprints/BP_FactoryCharacter` (`GameplayStatics.GetPlayerCharacter` 0)))
      (set `/Game/Blueprints/BP_FactoryCharacter.playerCarryState` "NewEnumerator0" _asbp_factory_character_2))))

(event `ChargeMechanicalObject`
  (bind _treadmillobj (`self.treadmillObj`))
  (if (`|EnumEquality` (`self.compartmentState`) "NewEnumerator1")
    (if (not (`self.charged?`))
      (`GameplayStatics.PlaySoundAtLocation` "/Game/Audio/SFX/Electricity___Shock.Electricity___Shock" (`SceneComponent.K2_GetComponentLocation` (`self.Box`)) (struct) 1.0 1.0 0.0 null null null null)
      (set `self.charged?` true)
      (if (`|EnumEquality` (`self.objectAttachment`) "NewEnumerator0")
        (set `/Game/Blueprints/MechanicalObjects/BP_Treadmill.splineIndex` 0 _treadmillobj)
        (`SceneComponent.K2_SetRelativeLocation` (`/Game/Blueprints/MechanicalObjects/BP_Treadmill.BigBattery` _treadmillobj) (`.Position` (break `SplinePoint` (`SplineComponent.GetSplinePointAt` (`/Game/Blueprints/MechanicalObjects/BP_Treadmill.Spline` _treadmillobj) 0 "Local"))) false false)
        (`GameplayStatics.PlaySoundAtLocation` "/Game/Audio/SFX/Conveyor_Belt__StartUp_.Conveyor_Belt__StartUp_" (`SceneComponent.K2_GetComponentLocation` (`self.Box`)) (struct) 1.0 1.0 0.0 null null null null)
        (bind _returnvalue (`GameplayStatics.SpawnSoundAtLocation` "/Game/Audio/SFX/Conveyor_Belt__Loop__v2.Conveyor_Belt__Loop__v2" (`SceneComponent.K2_GetComponentLocation` (`/Game/Blueprints/MechanicalObjects/BP_Treadmill.DefaultSceneRoot` _treadmillobj)) (struct) 1.0 1.0 0.0 null null))
        (`/Game/Blueprints/MechanicalObjects/BP_Treadmill.BatteryChargeCycle` _treadmillobj self)
        (elif (`|EnumEquality` (`self.objectAttachment`) "NewEnumerator1")
          (`/Game/Blueprints/MechanicalObjects/BP_HandyBot.ActivateRobot` (`self.handyBotObj`) self))))))

(event `StopTreadmill`
  (`AudioComponent.Stop` (stale `ChargeMechanicalObject` _returnvalue)))

(event `UnloadCompartment`
  (`SceneComponent.SetVisibility` (`self.PSCP_Game_Jam_battery`) false false)
  (set `self.compartmentState` "NewEnumerator0")
  (bind _returnvalue (`|SpawnActorFromClass` "/Game/Blueprints/MechanicalObjects/BP_Battery.BP_Battery_C" (`KismetMathLibrary.MakeTransform` (`SceneComponent.K2_GetComponentLocation` (`self.Arrow`)) (struct) (2.0 2.0 2.0)) "Undefined" "MultiplyWithRoot" null null))
  (bind _staticmesh (`/Game/Blueprints/MechanicalObjects/BP_Battery.StaticMesh` _returnvalue))
  (`PrimitiveComponent.AddImpulseAtLocation` _staticmesh (* (`SceneComponent.GetForwardVector` (`self.Arrow`)) 1000.0) (`SceneComponent.K2_GetComponentLocation` _staticmesh) "None"))

(event `AttemptToCharge`
  (if (and (`self.redClampConnected?`) (`self.blackClampConnected?`))
    (if (not (`self.charged?`))
      (`self.ChargeMechanicalObject`))))

(fn `UserConstructionScript`)