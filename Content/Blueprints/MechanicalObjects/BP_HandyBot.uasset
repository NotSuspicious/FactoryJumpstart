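; BP_HandyBot is a battery-powered robot that hands a big battery from the previous treadmill to the next one.
; Activation raises its arm holder by timeline and starts a timer that powers it down and drains the compartment.
; While charged, a sphere overlap takes the battery, then recursive MoveComponentTo events turn the body and step the battery along spline points.
; Delivery sets the next treadmill's mesh, and a variant flag completes the final level trigger.
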(event `ActivateRobot`
  (params (batteryCompartment :type "/Game/Blueprints/MechanicalObjects/BP_BatteryCompartment Object Reference"))
  (set `self.charged?` true)
  (`self.PowerUp`)
  (`KismetSystemLibrary.K2_SetTimerDelegate` (delegate `PowerDown`) 8.0))

(event `PowerUp`
  (bind _armsholder (`self.ArmsHolder`))
  (bind (_relativelocation_x _relativelocation_y) (`KismetMathLibrary.BreakVector` (`SceneComponent.RelativeLocation` _armsholder)))
  (bind (_direction _newtrack_0) (`Timeline|Timeline` :!label _label)
    (:`Update`
      (`SceneComponent.K2_SetRelativeLocation` _armsholder (`KismetMathLibrary.MakeVector` (`KismetMathLibrary.Lerp` 0.0 -50.0 _newtrack_0) _relativelocation_y (`KismetMathLibrary.Lerp` 0.0 50.0 _newtrack_0)) false false))))

(event `PowerDown`
  (set `/Game/Blueprints/MechanicalObjects/BP_BatteryCompartment.charged?` false (stale `ActivateRobot` batteryCompartment))
  (set `self.charged?` false)
  (goto _label :!via `ReverseFromEnd`))

(event `OneTreadToTheNext(Battery)`
  (bind (_inputkey _position) (break `SplinePoint` (`SplineComponent.GetSplinePointAt` (`self.Spline`) (`self.splineIndex`) "Local")))
  (if (== (`self.splineIndex`) (`SplineComponent.GetNumberOfSplinePoints` (`self.Spline`)))
    (`self.TransferBattery`)
    (else
      (`KismetSystemLibrary.MoveComponentTo` (`self.BatteryHolder`) (`KismetMathLibrary.MakeVector` (.x _position) (.y _position) (+ (.z _position) 50.0)) (struct) false false 0.5 true)
      (`/Engine/EditorBlueprintResources/StandardMacros.IncrementInt` (`self.splineIndex`)
        (:`  `
          (`self.OneTreadToTheNext(Battery)`))))))

(event `OneTreadToTheNext`
  (bind (_returnvalue_roll _returnvalue_pitch _returnvalue_yaw) (`KismetMathLibrary.BreakRotator` (`KismetMathLibrary.FindLookAtRotation` (`SceneComponent.RelativeLocation` (`self.Body`)) (`SplineComponent.GetLocationAtSplinePoint` (`self.Spline`) (`self.splineIndex`) "Local"))))
  (if (== (`self.splineIndex`) (`SplineComponent.GetNumberOfSplinePoints` (`self.Spline`)))
    (`self.ResetTurn`)
    (else
      (`KismetSystemLibrary.MoveComponentTo` (`self.Body`) (0.0 0.0 0.0) (`KismetMathLibrary.MakeRotator` 0.0 0.0 (+ _returnvalue_yaw -180.0)) false false 0.35 true)
      (`self.OneTreadToTheNext`))))

(event `TransferBattery`
  (bind _batteryholder (`self.BatteryHolder`))
  (set `self.carryBatteryState` "NewEnumerator0")
  (`StaticMeshComponent.SetStaticMesh` (`/Game/Blueprints/MechanicalObjects/BP_Treadmill.BigBattery` (`self.newTreadmill`)) "/Engine/BasicShapes/BigBattery.BigBattery")
  (`StaticMeshComponent.SetStaticMesh` _batteryholder null)
  (`SceneComponent.K2_SetRelativeLocation` _batteryholder (100.0 0.0 100.0) false false)
  (if (`self.isVariant?`)
    (set `/Game/Blueprints/WinCondition/BP_LevelCompleteTrigger.levelComplete?` true (`self.finalLevelTrigger`))))

(event `ResetTurn`
  (bind (_returnvalue_roll _returnvalue_pitch _returnvalue_yaw) (`KismetMathLibrary.BreakRotator` (`KismetMathLibrary.FindLookAtRotation` (`SceneComponent.RelativeLocation` (`self.Body`)) (`SplineComponent.GetLocationAtSplinePoint` (`self.Spline`) (`self.splineIndex`) "Local"))))
  (bind (_returnvalue_roll_2 _returnvalue_pitch_2 _returnvalue_yaw_2) (`KismetMathLibrary.BreakRotator` (`KismetMathLibrary.FindLookAtRotation` (`SceneComponent.RelativeLocation` (`self.Body`)) (`SplineComponent.GetLocationAtSplinePoint` (`self.Spline`) (`self.splineIndex`) "Local"))))
  (if (== (`self.splineIndex`) 0)
    (`KismetSystemLibrary.MoveComponentTo` (`self.Body`) (0.0 0.0 0.0) (`KismetMathLibrary.MakeRotator` 0.0 0.0 (+ _returnvalue_yaw_2 -180.0)) false false 0.5)
    (else
      (`KismetSystemLibrary.MoveComponentTo` (`self.Body`) (0.0 0.0 0.0) (`KismetMathLibrary.MakeRotator` 0.0 0.0 (+ _returnvalue_yaw -180.0)) false false 0.5)
      (`/Engine/EditorBlueprintResources/StandardMacros.DecrementInt` (`self.splineIndex`)
        (:`  `
          (`self.ResetTurn`))))))

(event `self.Sphere.OnComponentBeginOverlap`
  (params (OverlappedComponent :type "PrimitiveComponent Object Reference") (OtherActor :type "Actor Object Reference") (OtherComp :type "PrimitiveComponent Object Reference") (OtherBodyIndex :type Integer) (bFromSweep :type Boolean) (SweepResult :type "HitResult Structure (by ref)"))
  (bind _previoustreadmill (`self.previousTreadmill`))
  (bind _bigbattery (`/Game/Blueprints/MechanicalObjects/BP_Treadmill.BigBattery` _previoustreadmill))
  (if (`self.charged?`)
    (if (== _bigbattery OtherComp)
      (set `/Game/Blueprints/MechanicalObjects/BP_Treadmill.carryBatteryState` "NewEnumerator0" _previoustreadmill)
      (`StaticMeshComponent.SetStaticMesh` _bigbattery null)
      (`StaticMeshComponent.SetStaticMesh` (`self.BatteryHolder`) "/Engine/BasicShapes/BigBattery.BigBattery")
      (`self.OneTreadToTheNext`)
      (`SceneComponent.K2_SetRelativeLocation` (`self.BatteryHolder`) (`KismetMathLibrary.MakeVector` (.x (`SplineComponent.GetLocationAtSplinePoint` (`self.Spline`) 0 "Local")) (.y (`SplineComponent.GetLocationAtSplinePoint` (`self.Spline`) 0 "Local")) (+ (.z (`SplineComponent.GetLocationAtSplinePoint` (`self.Spline`) 0 "Local")) 50.0)) false false)
      (`self.OneTreadToTheNext(Battery)`))))

(fn `UserConstructionScript`)