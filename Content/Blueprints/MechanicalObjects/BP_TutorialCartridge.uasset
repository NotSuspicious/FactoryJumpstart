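; BP_TutorialCartridge is an actor that supplies tutorial text to the factory character.
; Its sphere overlap sets itself as the BP_FactoryCharacter's TutorialCartridge reference on entry and clears it on exit.
; PrintDialogue looks up its TutorialTextName row in DT_TutorialText, then shows the passed-in widget and updates its text when the row is found.
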(event `self.Sphere.OnComponentBeginOverlap`
  (params (OverlappedComponent :type "PrimitiveComponent Object Reference") (OtherActor :type "Actor Object Reference") (OtherComp :type "PrimitiveComponent Object Reference") (OtherBodyIndex :type Integer) (bFromSweep :type Boolean) (SweepResult :type "HitResult Structure (by ref)"))
  (bind _asbp_factory_character (cast `/Game/Blueprints/BP_FactoryCharacter` OtherActor))
  (set `/Game/Blueprints/BP_FactoryCharacter.tutorialCartridge` self _asbp_factory_character))

(event `self.Sphere.OnComponentEndOverlap`
  (params (OverlappedComponent :type "PrimitiveComponent Object Reference") (OtherActor :type "Actor Object Reference") (OtherComp :type "PrimitiveComponent Object Reference") (OtherBodyIndex :type Integer))
  (bind _asbp_factory_character (cast `/Game/Blueprints/BP_FactoryCharacter` OtherActor))
  (set `/Game/Blueprints/BP_FactoryCharacter.tutorialCartridge` null _asbp_factory_character))

(event `PrintDialogue`
  (params (tutorialWidget :type "/Game/Blueprints/UI/UW_DialogueUI Object Reference"))
  (bind _returnvalue (`|GetDataTableRow` "/Game/DataTables/DT_TutorialText.DT_TutorialText" (`self.tutorialTextName`))
    (:`then`
      (`Widget.SetVisibility` tutorialWidget "Visible")
      (`/Game/Blueprints/UI/UW_DialogueUI.UpdateText` tutorialWidget (`.TutorialText_3_D86508A745F78590B4099696CB7D3ED6` (break `/Game/Structs/S_TutorialDialogue` _returnvalue))))))

(fn `UserConstructionScript`)