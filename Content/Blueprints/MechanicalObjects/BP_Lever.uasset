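; BP_Lever is a lever that a BP_FactoryCharacter can use to eject the contents of a linked BatteryCompartment.
; A sphere overlap sets or clears the character's CanUseLever flag and CurrentLever reference.
; ActivateEject checks the compartment state, swings the mesh pitch on a timeline, then calls UnloadCompartment and ReverseLever.
; ReverseLever runs a second timeline backwards, but its fixed lerp alpha holds the mesh at the start angle rather than animating it.
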(event `ActivateEject`
  (bind _staticmesh (`self.StaticMesh`))
  (bind (_relativerotation_roll _relativerotation_pitch _relativerotation_yaw) (`KismetMathLibrary.BreakRotator` (`SceneComponent.RelativeRotation` _staticmesh)))
  (if (`|EnumEquality` (`/Game/Blueprints/MechanicalObjects/BP_BatteryCompartment.compartmentState` (`self.batteryCompartment`)) "NewEnumerator1")
    (bind (_direction _newtrack_0) (`Timeline|Timeline` :!via `PlayFromStart`)
      (:`Update`
        (`SceneComponent.K2_SetRelativeRotation` _staticmesh (`KismetMathLibrary.MakeRotator` _relativerotation_roll (`KismetMathLibrary.Lerp` 45.0 -45.0 _newtrack_0) _relativerotation_yaw) false false))
      (:`Finished`
        (`/Game/Blueprints/MechanicalObjects/BP_BatteryCompartment.UnloadCompartment` (`self.batteryCompartment`))
        (`self.ReverseLever`)))))

(event `ReverseLever`
  (bind _staticmesh (`self.StaticMesh`))
  (bind (_relativerotation_roll _relativerotation_pitch _relativerotation_yaw) (`KismetMathLibrary.BreakRotator` (`SceneComponent.RelativeRotation` _staticmesh)))
  (`Timeline|Timeline_0` :!via `ReverseFromEnd`
    (:`Update`
      (`SceneComponent.K2_SetRelativeRotation` _staticmesh (`KismetMathLibrary.MakeRotator` _relativerotation_roll (`KismetMathLibrary.Lerp` 45.0 -45.0) _relativerotation_yaw) false false))))

(event `self.Sphere.OnComponentBeginOverlap`
  (params (OverlappedComponent :type "PrimitiveComponent Object Reference") (OtherActor :type "Actor Object Reference") (OtherComp :type "PrimitiveComponent Object Reference") (OtherBodyIndex :type Integer) (bFromSweep :type Boolean) (SweepResult :type "HitResult Structure (by ref)"))
  (bind _asbp_factory_character (cast `/Game/Blueprints/BP_FactoryCharacter` OtherActor))
  (set `/Game/Blueprints/BP_FactoryCharacter.canUseLever?` true _asbp_factory_character)
  (set `/Game/Blueprints/BP_FactoryCharacter.currentLever` self _asbp_factory_character))

(event `self.Sphere.OnComponentEndOverlap`
  (params (OverlappedComponent :type "PrimitiveComponent Object Reference") (OtherActor :type "Actor Object Reference") (OtherComp :type "PrimitiveComponent Object Reference") (OtherBodyIndex :type Integer))
  (bind _asbp_factory_character (cast `/Game/Blueprints/BP_FactoryCharacter` OtherActor))
  (set `/Game/Blueprints/BP_FactoryCharacter.canUseLever?` false _asbp_factory_character)
  (set `/Game/Blueprints/BP_FactoryCharacter.currentLever` null _asbp_factory_character))

(fn `UserConstructionScript`)