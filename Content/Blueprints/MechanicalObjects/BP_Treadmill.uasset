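; BP_Treadmill is a mechanical conveyor that carries a big battery along a spline while driven by a battery compartment.
; BeginPlay snaps the battery to the first point and, depending on CarryBatteryState, resets its mesh.
; BatteryChargeCycle sets the shared material's Speed parameter and re-calls itself after each one-second move to the next point.
; Reaching the end clears the compartment's charge and stops the treadmill; a transfer event also stops it and blocks further cycles.
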(event `self.ReceiveBeginPlay`
  (bind (_inputkey _position) (break `SplinePoint` (`SplineComponent.GetSplinePointAt` (`self.Spline`) 0 "Local")))
  (`SceneComponent.K2_SetRelativeLocation` (`self.BigBattery`) (`KismetMathLibrary.MakeVector` (.x _position) (.y _position) (.z _position)) false false)
  (if (not (`|EnumEquality` (`self.carryBatteryState`) "NewEnumerator1"))
    (`StaticMeshComponent.SetStaticMesh` (`self.BigBattery`) null)))

(event `BatteryChargeCycle`
  (params (batteryCompartment :type "/Game/Blueprints/MechanicalObjects/BP_BatteryCompartment Object Reference"))
  (bind _splineindex (`self.splineIndex`))
  (bind (_inputkey _position) (break `SplinePoint` (`SplineComponent.GetSplinePointAt` (`self.Spline`) _splineindex "Local")))
  (if (not (`self.batteryTransfered`))
    (bind _returnvalue (`MaterialInstanceDynamic.K2_GetScalarParameterValue` (`SharedMaterialController.SharedMaterial` (`self.MaterialController`)) "Speed"))
    (if (not (`KismetMathLibrary.NearlyEqual_FloatFloat` _returnvalue 1.0))
      (`MaterialInstanceDynamic.SetScalarParameterValue` (`SharedMaterialController.SharedMaterial` (`self.MaterialController`)) "Speed" 1.0))
    (if (== (`SplineComponent.GetNumberOfSplinePoints` (`self.Spline`)) _splineindex)
      (set `/Game/Blueprints/MechanicalObjects/BP_BatteryCompartment.charged?` false batteryCompartment)
      (`MaterialInstanceDynamic.SetScalarParameterValue` (`SharedMaterialController.SharedMaterial` (`self.MaterialController`)) "Speed" 0.0)
      (`/Game/Blueprints/MechanicalObjects/BP_BatteryCompartment.StopTreadmill` batteryCompartment)
      (else
        (`KismetSystemLibrary.MoveComponentTo` (`self.BigBattery`) (`KismetMathLibrary.MakeVector` (.x _position) (.y _position) (.z _position)) (struct) false false 1.0)
        (`/Engine/EditorBlueprintResources/StandardMacros.IncrementInt` (`self.splineIndex`)
          (:`  `
            (`self.BatteryChargeCycle` batteryCompartment)))))))

(event `StopTreadmillMaterialAfterTransfer`
  (`MaterialInstanceDynamic.SetScalarParameterValue` (`SharedMaterialController.SharedMaterial` (`self.MaterialController`)) "Speed" 0.0)
  (set `self.batteryTransfered` true)
  (`/Game/Blueprints/MechanicalObjects/BP_BatteryCompartment.StopTreadmill` (stale `BatteryChargeCycle` batteryCompartment)))

(fn `UserConstructionScript`)