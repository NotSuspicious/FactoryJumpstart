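; Level exit door that becomes usable by the player once its FinishLevelTrigger reports the level complete.
; Capsule overlap registers the door as the BP_FactoryCharacter's LevelExit and shows a widget, hidden at BeginPlay; leaving clears both.
; NextLevel rechecks completion but only prints a message, with no level loading yet.
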(event `self.ReceiveBeginPlay`
  (`SceneComponent.SetVisibility` (`self.Widget`) false false))

(event `self.Capsule.OnComponentBeginOverlap`
  (params (OverlappedComponent :type "PrimitiveComponent Object Reference") (OtherActor :type "Actor Object Reference") (OtherComp :type "PrimitiveComponent Object Reference") (OtherBodyIndex :type Integer) (bFromSweep :type Boolean) (SweepResult :type "HitResult Structure (by ref)"))
  (if (`/Game/Blueprints/WinCondition/BP_LevelCompleteTrigger.levelComplete?` (`self.finishLevelTrigger`))
    (bind _asbp_factory_character (cast `/Game/Blueprints/BP_FactoryCharacter` OtherActor))
    (set `/Game/Blueprints/BP_FactoryCharacter.levelExit` self _asbp_factory_character)
    (`SceneComponent.SetVisibility` (`self.Widget`) true false)))

(event `self.Capsule.OnComponentEndOverlap`
  (params (OverlappedComponent :type "PrimitiveComponent Object Reference") (OtherActor :type "Actor Object Reference") (OtherComp :type "PrimitiveComponent Object Reference") (OtherBodyIndex :type Integer))
  (if (`/Game/Blueprints/WinCondition/BP_LevelCompleteTrigger.levelComplete?` (`self.finishLevelTrigger`))
    (bind _asbp_factory_character (cast `/Game/Blueprints/BP_FactoryCharacter` OtherActor))
    (set `/Game/Blueprints/BP_FactoryCharacter.levelExit` null _asbp_factory_character)
    (`SceneComponent.SetVisibility` (`self.Widget`) false false)))

(event `NextLevel`
  (if (`/Game/Blueprints/WinCondition/BP_LevelCompleteTrigger.levelComplete?` (`self.finishLevelTrigger`))
    (`KismetSystemLibrary.PrintString` "Heading To Next Level")))

(fn `UserConstructionScript`)