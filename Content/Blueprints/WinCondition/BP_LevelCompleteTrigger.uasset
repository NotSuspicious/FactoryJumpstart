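; BP_LevelCompleteTrigger is a win-condition volume that flags the level as complete when the final treadmill's battery reaches it.
; A sphere overlap event sets LevelComplete if the overlapping component is FinalTreadmill's BigBattery.
; A looping half-second timer also polls overlapping BP_Treadmill actors and completes the level if FinalTreadmill is among them in a specific CarryBatteryState.
; Both paths only set the flag and print debug text.
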(event `self.Sphere.OnComponentBeginOverlap`
  (params (OverlappedComponent :type "PrimitiveComponent Object Reference") (OtherActor :type "Actor Object Reference") (OtherComp :type "PrimitiveComponent Object Reference") (OtherBodyIndex :type Integer) (bFromSweep :type Boolean) (SweepResult :type "HitResult Structure (by ref)"))
  (if (== (`/Game/Blueprints/MechanicalObjects/BP_Treadmill.BigBattery` (`self.finalTreadmill`)) OtherComp)
    (set `self.levelComplete?` true)
    (`KismetSystemLibrary.PrintString` "FINISH")))

(event `self.ReceiveBeginPlay`
  (`KismetSystemLibrary.K2_SetTimerDelegate` (delegate `CheckOverlapping`) 0.5 true))

(event `CheckOverlapping`
  (bind _finaltreadmill (`self.finalTreadmill`))
  (for _array_element (`PrimitiveComponent.GetOverlappingActors` (`self.Sphere`) "/Game/Blueprints/MechanicalObjects/BP_Treadmill.BP_Treadmill_C")
    (`KismetSystemLibrary.PrintString` (`KismetSystemLibrary.GetDisplayName` _array_element))
    (if (== _finaltreadmill _array_element)
      (if (`|EnumEquality` (`/Game/Blueprints/MechanicalObjects/BP_Treadmill.carryBatteryState` _finaltreadmill) "NewEnumerator1")
        (set `self.levelComplete?` true)
        (`KismetSystemLibrary.PrintString` "FINISH")))))

(fn `UserConstructionScript`)